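; BP_Enemy is a melee enemy that chases the player and deals contact damage.
; Pawn sensing triggers AI MoveTo toward the player, then plays an attack montage on arrival, gated by CanAttack for the montage's length.
; Damage is separate from the animation: capsule overlap starts a looping timer that damages the overlapping actor with a sound, cleared on end overlap.
; Received damage reduces clamped health, and at zero it enables physics before delayed destruction.
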(event `self.PawnSensing.OnSeePawn`
  (params (Pawn :type "Pawn Object Reference"))
  ;[1 1 1] Track and follow the player
  (set `self.SeenPlayer` true)
  (`self.Follow Player`))

(event `Follow Player`
  ;[1 1 1] Track and follow the player
  (set `self.CanAttack` true)
  (if (`self.SeenPlayer`)
    (`|AIMoveTo` self (0.0 0.0 0.0) (`GameplayStatics.GetPlayerCharacter` 0)
      (:`OnSuccess`
        (if (`self.CanAttack`)
          (set `self.CanAttack` false)
          (bind _returnvalue (`self.PlayAnimMontage` "/Game/FreeAnimationLibrary/Animations/Counter-Finisher/EnemyAttack.EnemyAttack"))
          (`KismetSystemLibrary.Delay` _returnvalue)
          (set `self.CanAttack` true))))))

(event `self.Capsule.OnComponentBeginOverlap`
  (params (OverlappedComponent :type "PrimitiveComponent Object Reference") (OtherActor :type "Actor Object Reference") (OtherComp :type "PrimitiveComponent Object Reference") (OtherBodyIndex :type Integer) (bFromSweep :type Boolean) (SweepResult :type "HitResult Structure (by ref)"))
  ;[1 1 1] Attack the player
  (set `self.PlayerClose` true)
  (bind _returnvalue (`KismetSystemLibrary.K2_SetTimerDelegate` (delegate `DamagePlayer`) 0.4 true))
  (set `self.DamageTimer` _returnvalue))

(event `DamagePlayer`
  ;[1 1 1] Attack the player
  (`GameplayStatics.ApplyDamage` (stale `self.Capsule.OnComponentBeginOverlap` OtherActor) 20.0)
  (`GameplayStatics.PlaySoundAtLocation` "/Game/Sound/458867__raclure__damage-sound-effect.458867__raclure__damage-sound-effect" (0.0 0.0 0.0) (struct) 1.0 1.0 0.0 null null null null))

(event `self.Capsule.OnComponentEndOverlap`
  (params (OverlappedComponent :type "PrimitiveComponent Object Reference") (OtherActor :type "Actor Object Reference") (OtherComp :type "PrimitiveComponent Object Reference") (OtherBodyIndex :type Integer))
  ;[1 1 1] Attack the player
  (set `self.PlayerClose` false)
  (`KismetSystemLibrary.K2_ClearAndInvalidateTimerHandle` (`self.DamageTimer`)))

(event `self.ReceiveAnyDamage`
  (params (Damage :type "Float (single-precision)") (DamageType :type "DamageType Object Reference") (InstigatedBy :type "Controller Object Reference") (DamageCauser :type "Actor Object Reference"))
  (if (not (`self.Dead`))
    (bind _output_get (set `self.CurrentHealth` (`KismetMathLibrary.FClamp` (- (`self.CurrentHealth`) Damage) 0.0 50.0)))
    (if (== _output_get 0.0)
      (`PrimitiveComponent.SetSimulatePhysics` (`self.Mesh`) true)
      (`PrimitiveComponent.SetSimulatePhysics` (`self.Capsule`) true)
      (`KismetSystemLibrary.Delay` 1.0)
      (`self.K2_DestroyActor`))))

(fn `UserConstructionScript`)