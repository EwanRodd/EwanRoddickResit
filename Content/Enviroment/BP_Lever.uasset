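; BP_Lever is an environment lever that opens a linked gate and shows a gate-points widget when the first-person character is nearby.
; Entering the PlayerNear volume registers the lever on the character and creates the WBP_GatePoints widget on screen.
; Leaving clears that reference and removes the widget.
; The Opening event, which has no caller in this Blueprint, calls OpenGate on the referenced Gate.
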(event `self.PlayerNear.OnComponentBeginOverlap`
  (params (OverlappedComponent :type "PrimitiveComponent Object Reference") (OtherActor :type "Actor Object Reference") (OtherComp :type "PrimitiveComponent Object Reference") (OtherBodyIndex :type Integer) (bFromSweep :type Boolean) (SweepResult :type "HitResult Structure (by ref)"))
  (bind _asbp_first_person_character (cast `/Game/FirstPerson/Blueprints/BP_FirstPersonCharacter` OtherActor))
  (set `/Game/FirstPerson/Blueprints/BP_FirstPersonCharacter.Lever` self _asbp_first_person_character)
  (bind _returnvalue (`|CreateWidget` "/Game/UI/WBP_GatePoints.WBP_GatePoints_C"))
  (bind _output_get (set `self.GatePointsText` _returnvalue))
  (`UserWidget.AddToViewport` _returnvalue 0)
  (`UserWidget.AddToViewport` _output_get 0))

(event `self.PlayerNear.OnComponentEndOverlap`
  (params (OverlappedComponent :type "PrimitiveComponent Object Reference") (OtherActor :type "Actor Object Reference") (OtherComp :type "PrimitiveComponent Object Reference") (OtherBodyIndex :type Integer))
  (bind _gatepointstext (`self.GatePointsText`))
  (bind _asbp_first_person_character (cast `/Game/FirstPerson/Blueprints/BP_FirstPersonCharacter` OtherActor))
  (set `/Game/FirstPerson/Blueprints/BP_FirstPersonCharacter.Lever` null _asbp_first_person_character)
  (`/Engine/EditorBlueprintResources/StandardMacros.IsValid` _gatepointstext
    (:`Is Valid`
      (`Widget.RemoveFromParent` _gatepointstext))))

(event `Opening`
  (`/Game/Enviroment/BP_Gate.Open Gate` (`self.Gate`)))

(fn `UserConstructionScript`)