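; BP_TrapLever is an environment lever that lets the first-person player activate a linked trap.
; Its overlap sphere registers the lever on BP_FirstPersonCharacter and shows a WBP_TrapText widget, then clears the reference and removes the widget on exit.
; ActivateTrap, which nothing in this Blueprint calls, forwards to SpinTrap on the referenced Trap.
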(event `Activate Trap`
  (`/Game/Traps/BP_Trap.Spin Trap` (`self.Trap`)))

(event `self.Sphere.OnComponentBeginOverlap`
  (params (OverlappedComponent :type "PrimitiveComponent Object Reference") (OtherActor :type "Actor Object Reference") (OtherComp :type "PrimitiveComponent Object Reference") (OtherBodyIndex :type Integer) (bFromSweep :type Boolean) (SweepResult :type "HitResult Structure (by ref)"))
  (bind _asbp_first_person_character (cast `/Game/FirstPerson/Blueprints/BP_FirstPersonCharacter` OtherActor))
  (set `/Game/FirstPerson/Blueprints/BP_FirstPersonCharacter.TrapLever` self _asbp_first_person_character)
  (bind _returnvalue (`|CreateWidget` "/Game/UI/WBP_TrapText.WBP_TrapText_C"))
  (bind _output_get (set `self.TrapText` _returnvalue))
  (`UserWidget.AddToViewport` _output_get 0)
  (`UserWidget.AddToViewport` _returnvalue 0))

(event `self.Sphere.OnComponentEndOverlap`
  (params (OverlappedComponent :type "PrimitiveComponent Object Reference") (OtherActor :type "Actor Object Reference") (OtherComp :type "PrimitiveComponent Object Reference") (OtherBodyIndex :type Integer))
  (bind _asbp_first_person_character (cast `/Game/FirstPerson/Blueprints/BP_FirstPersonCharacter` OtherActor))
  (set `/Game/FirstPerson/Blueprints/BP_FirstPersonCharacter.TrapLever` null _asbp_first_person_character)
  (`Widget.RemoveFromParent` (`self.TrapText`)))

(fn `UserConstructionScript`)