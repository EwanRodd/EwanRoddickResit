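; BP_Button is an interactable button that opens a linked second gate.
; Its Sphere overlap registers the button on BP_FirstPersonCharacter and shows a WBP_SecondGate widget, then clears the reference and removes the widget when the character leaves.
; The PressGateButton event calls OpenSecondGate on the SecondGate reference, with no caller inside this Blueprint.
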(event `self.Sphere.OnComponentBeginOverlap`
  (params (OverlappedComponent :type "PrimitiveComponent Object Reference") (OtherActor :type "Actor Object Reference") (OtherComp :type "PrimitiveComponent Object Reference") (OtherBodyIndex :type Integer) (bFromSweep :type Boolean) (SweepResult :type "HitResult Structure (by ref)"))
  (bind _asbp_first_person_character (cast `/Game/FirstPerson/Blueprints/BP_FirstPersonCharacter` OtherActor))
  (set `/Game/FirstPerson/Blueprints/BP_FirstPersonCharacter.Button` self _asbp_first_person_character)
  (bind _returnvalue (`|CreateWidget` "/Game/UI/WBP_SecondGate.WBP_SecondGate_C"))
  (bind _output_get (set `self.Second Gate Text` _returnvalue))
  (`UserWidget.AddToViewport` _output_get 0)
  (`UserWidget.AddToViewport` _returnvalue 0))

(event `self.Sphere.OnComponentEndOverlap`
  (params (OverlappedComponent :type "PrimitiveComponent Object Reference") (OtherActor :type "Actor Object Reference") (OtherComp :type "PrimitiveComponent Object Reference") (OtherBodyIndex :type Integer))
  (bind _second_gate_text (`self.Second Gate Text`))
  (bind _asbp_first_person_character (cast `/Game/FirstPerson/Blueprints/BP_FirstPersonCharacter` OtherActor))
  (set `/Game/FirstPerson/Blueprints/BP_FirstPersonCharacter.Button` null _asbp_first_person_character)
  (`/Engine/EditorBlueprintResources/StandardMacros.IsValid` _second_gate_text
    (:`Is Valid`
      (`Widget.RemoveFromParent` _second_gate_text))))

(event `Press Gate Button`
  (`/Game/Enviroment/BP_SecondGate.Open Second Gate` (`self.SecondGate`)))

(fn `UserConstructionScript`)